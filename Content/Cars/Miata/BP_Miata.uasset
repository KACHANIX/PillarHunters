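; Drivable Miata with hand-built vehicle physics, engine sound, camera control and debug readouts.
; Each tick, four line traces drive spring-damper suspension, whose load scales longitudinal force and clamps lateral force applied to the body.
; Throttle feeds a torque-curve engine and timed gearbox that spin the rear wheels, capped by engine speed.
; Wheel spin is visual only: longitudinal force comes from the Forward input axis, not drivetrain torque.
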(event `self.ReceiveBeginPlay`
  (`self.SetUnitMultipliers`)
  (`self.InitComponents`)
  (`self.InitSuspensionRay`)
  (`self.InitSuspension`)
  (`self.SetGearNumbers`)
  (`self.GetWheelInertia`)
  (bind _returnvalue (`|CreateWidget` "/Game/HUD/RPM.RPM_C"))
  (`UserWidget.AddToViewport` _returnvalue 0))

(event `self.ReceiveTick`
  (params (DeltaSeconds :type "Float (single-precision)"))
  (set `self.DeltaT` DeltaSeconds)
  (`self.GetRearWheelsTorque`)
  (`self.WheelAcceleration`)
  (`self.SuspensionRay`)
  (`self.UpdateSuspensionLength`)
  (`self.GetSuspensionForce`)
  (`self.ApplySuspensionForce`)
  (`self.UpdateWheelLocation`)
  (`self.CameraMovement`)
  (`self.GetWheelLinearVelocityLocal`)
  (`self.GetWheelForce`)
  (`self.ApplyWheelForce`)
  (`self.DrawDebugForces`)
  (`self.SetEngineSound`)
  (for _index (range 4)
    (`SceneComponent.K2_AddLocalRotation` (select `int` _index :`0` (`self.FL_Wheel`) :`1` (`self.FR_Wheel`) :`2` (`self.RL_Wheel`) :`3` (`self.RR_Wheel`)) (`KismetMathLibrary.MakeRotator` 0.0 (* (`KismetMathLibrary.RadiansToDegrees` (`|GetArrayItem` (`self.WheelAngularVelocity`) _index)) (`self.DeltaT`))) false false)
    (`KismetSystemLibrary.PrintString` (`KismetStringLibrary.Conv_DoubleToString` (`|GetArrayItem` (`self.WheelAngularVelocity`) _index)) true false (struct :`R` 0.771037 :`G` 0.234375 :`B` 1.0 :`A` 1.0) 0.0)))

(event `InputAxis|Right`
  (params (AxisValue :type "Float (single-precision)"))
  (`self.SetSteeringAngle` AxisValue))

(event `InputAxis|Forward`
  (params (AxisValue :type "Float (single-precision)")))

(event `InputAxis|Throttle`
  (params (AxisValue :type "Float (single-precision)"))
  (`self.GetThrottle` AxisValue)
  (`self.SetEngineRPM`))

(event `Key|LeftMouseButton`
  (params (Key :type "Key Structure"))
  (:`Pressed`
    (if (!= (`self.Gear`) 6)
      (set `self.NextGear` (+ (`self.Gear`) 1))
      (set `self.Gear` 1)
      (set `self.TotalTransmissionRatio` 0.0)
      (`KismetSystemLibrary.Delay` (`self.GearShiftTime`))
      (set `self.Gear` (`KismetMathLibrary.Min` (`self.NextGear`) (`self.GearNumbers`)))
      (`self.SetTotalTransmissionRatio`))))

(event `Key|RightMouseButton`
  (params (Key :type "Key Structure"))
  (:`Pressed`
    (if (!= (`self.Gear`) 0)
      (set `self.NextGear` (- (`self.Gear`) 1))
      (set `self.Gear` 1)
      (set `self.TotalTransmissionRatio` 0.0)
      (`KismetSystemLibrary.Delay` (`self.GearShiftTime`))
      (set `self.Gear` (`KismetMathLibrary.Max` (`self.NextGear`)))
      (`self.SetTotalTransmissionRatio`))))

(event `Key|R`
  (params (Key :type "Key Structure"))
  (bind _miata_body (`self.miata_body`))
  (bind (_returnvalue_x _returnvalue_y _returnvalue_z) (`KismetMathLibrary.BreakVector` (`SceneComponent.K2_GetComponentLocation` _miata_body)))
  (:`Pressed`
    (`SceneComponent.K2_SetWorldLocation` _miata_body (`KismetMathLibrary.MakeVector` _returnvalue_x _returnvalue_y (+ _returnvalue_z 200.0)) false false)))

(event `Key|Q`
  (params (Key :type "Key Structure"))
  (:`Pressed`
    (`SceneComponent.K2_SetWorldLocation` (`self.miata_body`) (210.0 0.0 290.0) false false)))

(event `Key|Tab`
  (params (Key :type "Key Structure"))
  (:`Pressed`
    (bind _isa (`/Engine/EditorBlueprintResources/StandardMacros.FlipFlop`)
      (:`A`
        _)
      (:`B`
        _))
    (set `self.DebugF` _isa)))

(fn `ApplySuspensionForce`
  (for _index (range 4)
    (bind _output (`|GetArrayItem` (`self.CupComponent`) _index))
    (`PrimitiveComponent.AddForceAtLocation` (`self.miata_body`) (* (`SceneComponent.GetUpVector` _output) (* (`|GetArrayItem` (`self.SpringForces`) _index) 100.0)) (`SceneComponent.K2_GetComponentLocation` _output) "None")))

(fn `ApplyWheelForce`
  (for _index (range 4)
    (if (`|GetArrayItem` (`self.SurfaceContact`) _index)
      (bind _output (`|GetArrayItem` (`self.CupComponent`) _index))
      (bind (_output_bblockinghit _output_binitialoverlap _output_time _output_distance _output_location) (`GameplayStatics.BreakHitResult` (`|GetArrayItem` (`self.HitResult`) _index)))
      (`PrimitiveComponent.AddForceAtLocation` (`self.miata_body`) (* (+ (* (`SceneComponent.GetForwardVector` _output) (`|GetArrayItem` (`self.Fx_Wheel`) _index)) (* (`SceneComponent.GetRightVector` _output) (`|GetArrayItem` (`self.Fy_Wheel`) _index))) 100.0) _output_location "None"))))

(fn `CameraMovement`
  (bind _springarm (`self.SpringArm`))
  (bind (_returnvalue_roll _returnvalue_pitch _returnvalue_yaw) (`KismetMathLibrary.BreakRotator` (`SceneComponent.K2_GetComponentRotation` _springarm)))
  (`SceneComponent.K2_SetWorldRotation` _springarm (`KismetMathLibrary.MakeRotator` _returnvalue_roll (+ (`self.GetInputAxisKeyValue`) _returnvalue_pitch) (+ _returnvalue_yaw (`self.GetInputAxisKeyValue`))) false false))

(fn `DrawDebugForces`
  (if (`self.DebugF`)
    (for _index (range 4)
      (for _index_2 (range 3)
        (bind _returnvalue (`SceneComponent.K2_GetComponentLocation` (`|GetArrayItem` (`self.WheelComponent`) _index)))
        (bind _output (`|GetArrayItem` (`self.CupComponent`) _index))
        (`KismetSystemLibrary.DrawDebugLine` _returnvalue (+ _returnvalue (* (select `int` _index_2 :`0` (`SceneComponent.GetForwardVector` _output) :`1` (`SceneComponent.GetRightVector` _output) :`2` (`SceneComponent.GetUpVector` _output)) (/ (select `int` _index_2 :`0` (`|GetArrayItem` (`self.Fx_Wheel`) _index) :`1` (`|GetArrayItem` (`self.Fy_Wheel`) _index) :`2` (`|GetArrayItem` (`self.SpringForces`) _index)) 20.0))) (struct :`R` 0.073242 :`G` 0.840849 :`B` 0.9375 :`A` 1.0) 0.0 5.0)))))

(fn `GetRearWheelsTorque`
  (bind _totaltorque (`self.TotalTorque`))
  (bind _returnvalue (* (`KismetMathLibrary.FMax` (`self.EngineTorque`)) (`self.TotalTransmissionRatio`) 0.5))
  (`KismetArrayLibrary.Array_Set` _totaltorque 2 _returnvalue)
  (`KismetArrayLibrary.Array_Set` _totaltorque 3 _returnvalue)
  (for _index (range 4)
    (`KismetSystemLibrary.PrintString` (`KismetStringLibrary.Concat_StrStr` (select `int` _index :`0` "Torque FL " :`1` "Torque FR " :`2` "Torque RL " :`3` "Torque RR ") (`KismetStringLibrary.Conv_DoubleToString` (`|GetArrayItem` (`self.TotalTorque`) _index))) true true (struct :`R` 1.0 :`G` 0.033717 :`B` 0.21391 :`A` 1.0) 0.0)))

(fn `GetSuspensionForce`
  (for _index (range 4)
    (bind (_output_restlength _output_travel _output_stifness) (break `/Game/Cars/Miata/SuspensionStruct` (`|GetArrayItem` (`self.Suspension`) _index)))
    (bind _output (`|GetArrayItem` (`self.CurrentLength`) _index))
    (bind (_output_restlength_2 _output_travel_2 _output_stifness_2 _output_damper _output_springforcemin _output_springforcemax) (break `/Game/Cars/Miata/SuspensionStruct` (`|GetArrayItem` (`self.Suspension`) _index)))
    (bind _returnvalue (`KismetMathLibrary.FClamp` (+ (* _output_stifness (- _output_restlength _output)) (* (/ (- (`|GetArrayItem` (`self.PreviousLength`) _index) _output) (`self.DeltaT`)) _output_damper)) _output_springforcemin _output_springforcemax))
    (`KismetArrayLibrary.Array_Set` (`self.SpringForces`) _index _returnvalue)
    (`KismetArrayLibrary.Array_Set` (`self.PreviousLength`) _index (`|GetArrayItem` (`self.CurrentLength`) _index))
    (`KismetSystemLibrary.PrintString` (`KismetStringLibrary.Concat_StrStr` (select `int` _index :`0` "SpringForce_FL " :`1` "SpringForce_FR " :`2` "SpringForce_RL " :`3` "SpringForce_RR ") (`KismetStringLibrary.Conv_DoubleToString` _returnvalue)) false false (struct :`R` 1.0 :`B` 0.938498 :`A` 1.0) 0.0)))

(fn `GetThrottle`
  (params (InputPin :type "Float (double-precision)"))
  (bind _throttle (`self.Throttle`))
  (bind _deltat (`self.DeltaT`))
  (if (`self.ThrottleFilter`)
    (if (!= InputPin 0.0)
      (set `self.Throttle` (`KismetMathLibrary.FMin` (+ _throttle (* _deltat 2.0)) 1.0))
      (else
        (set `self.Throttle` (`KismetMathLibrary.FMax` (- _throttle (* _deltat 4.0))))))
    (else
      (set `self.Throttle` InputPin))))

(fn `GetWheelForce`
  (for _index (range 4)
    (if (`|GetArrayItem` (`self.SurfaceContact`) _index)
      (bind _output (`|GetArrayItem` (`self.SpringForces`) _index))
      (`KismetArrayLibrary.Array_Set` (`self.Fx_Wheel`) _index (* (`self.GetInputAxisValue`) _output 0.5))
      (bind (_output_x _output_y) (`KismetMathLibrary.BreakVector` (`|GetArrayItem` (`self.WheelLinearVelocityLocal`) _index)))
      (`KismetArrayLibrary.Array_Set` (`self.Fy_Wheel`) _index (`KismetMathLibrary.FClamp` (* _output_y _output -1.0) (* _output -1.0) _output))
      (else
        (`KismetArrayLibrary.Array_Set` (`self.Fx_Wheel`) _index)
        (`KismetArrayLibrary.Array_Set` (`self.Fy_Wheel`) _index)))))

(fn `GetWheelInertia`
  (for _index (range 4)
    (bind (_output_radius _output_mass) (break `/Game/Cars/Miata/WheelStruct` (`|GetArrayItem` (`self.Wheel`) _index)))
    (`KismetArrayLibrary.Array_Set` (`self.WheelInertia`) _index (* (`KismetMathLibrary.MultiplyMultiply_FloatFloat` (/ _output_radius 100.0) 2.0) _output_mass 0.5))))

(fn `GetWheelLinearVelocityLocal`
  (for _index (range 4)
    (bind _output (`|GetArrayItem` (`self.CupComponent`) _index))
    (bind _output_radius (break `/Game/Cars/Miata/WheelStruct` (`|GetArrayItem` (`self.Wheel`) _index)))
    (bind _returnvalue (`PrimitiveComponent.GetPhysicsLinearVelocityAtPoint` (`self.miata_body`) (- (`SceneComponent.K2_GetComponentLocation` (`|GetArrayItem` (`self.WheelComponent`) _index)) (* (`SceneComponent.GetUpVector` _output) _output_radius)) "None"))
    (`KismetArrayLibrary.Array_Set` (`self.WheelLinearVelocityLocal`) _index (`KismetMathLibrary.TransformDirection` (`KismetMathLibrary.InvertTransform` (`SceneComponent.K2_GetComponentToWorld` _output)) (/ _returnvalue 100.0)))))

(fn `InitComponents`
  (for _index (range 4)
    (`KismetArrayLibrary.Array_Set` (`self.CupComponent`) _index (select `int` _index :`0` (`self.FL_Cup`) :`1` (`self.FR_Cup`) :`2` (`self.RL_Cup`) :`3` (`self.RR_Cup`)))
    (`KismetArrayLibrary.Array_Set` (`self.WheelComponent`) _index (select `int` _index :`0` (`self.FL_Wheel`) :`1` (`self.FR_Wheel`) :`2` (`self.RL_Wheel`) :`3` (`self.RR_Wheel`)))))

(fn `InitSuspension`
  (for _index (range 4)
    (bind _restlength (break `/Game/Cars/Miata/SuspensionStruct` (`|GetArrayItem` (`self.Suspension`) _index)))
    (`KismetArrayLibrary.Array_Set` (`self.CurrentLength`) _index _restlength)
    (`KismetArrayLibrary.Array_Set` (`self.PreviousLength`) _index _restlength)))

(fn `InitSuspensionRay`
  (for _index (range 4)
    (bind (_output_restlength _output_travel) (break `/Game/Cars/Miata/SuspensionStruct` (`|GetArrayItem` (`self.Suspension`) _index)))
    (bind _output_radius (break `/Game/Cars/Miata/WheelStruct` (`|GetArrayItem` (`self.Wheel`) _index)))
    (`KismetArrayLibrary.Array_Set` (`self.RayLength`) _index (+ (+ _output_restlength _output_travel) _output_radius))))

(fn `SetEngineRPM`
  (bind (_engine_torque _engine_idles _engine_cutoff _engine_inertia _engine_backtorque) (break `/Game/Cars/Miata/EngineStruct` (`self.Engine`)))
  (bind (_engine_torque_2 _engine_idles_2 _engine_cutoff_2) (break `/Game/Cars/Miata/EngineStruct` (`self.Engine`)))
  (bind _rpm_rad_multiplier (`self.RPM_RAD_multiplier`))
  (bind _throttle (`self.Throttle`))
  (bind _output_get (set `self.EngineTorque` (`KismetMathLibrary.Lerp` _engine_backtorque (* (`CurveFloat.GetFloatValue` _engine_torque (`self.EngineRPM`)) _throttle) _throttle)))
  (bind _output_get_2 (set `self.EngineAngularVelocity` (`KismetMathLibrary.FClamp` (+ (`self.EngineAngularVelocity`) (* (/ _output_get _engine_inertia) (`self.DeltaT`))) (* _rpm_rad_multiplier _engine_idles_2) (* _rpm_rad_multiplier _engine_cutoff_2))))
  (bind _output_get_3 (set `self.EngineRPM` (* _output_get_2 (`self.RAD_RPM_multiplier`))))
  (`KismetSystemLibrary.PrintString` (`KismetStringLibrary.Concat_StrStr` "RPM= " (`KismetStringLibrary.Conv_DoubleToString` _output_get_3)) true false (struct :`R` 1.0 :`B` 0.774798 :`A` 1.0) 0.0)
  (`KismetSystemLibrary.PrintString` (`KismetStringLibrary.Concat_StrStr` "Torque= " (`KismetStringLibrary.Conv_DoubleToString` (`self.EngineTorque`))) true false (struct :`R` 1.0 :`B` 0.696258 :`A` 1.0) 0.0))

(fn `SetEngineSound`
  (bind _audio (`self.Audio`))
  (`AudioComponent.SetFloatParameter` _audio "EngineRPM" (`self.EngineRPM`))
  (`AudioComponent.SetPitchMultiplier` _audio 1.0)
  (`AudioComponent.SetBoolParameter` _audio "t" (> (`self.Throttle`) 0.0)))

(fn `SetGearNumbers`
  (set `self.GearNumbers` (- (`KismetArrayLibrary.Array_Length` (`self.GearRatio`)) 1)))

(fn `SetSteeringAngle`
  (params (A :type "Float (double-precision)"))
  (bind _steeringangle (`self.SteeringAngle`))
  (bind _steeringanglemax (`self.SteeringAngleMax`))
  (if (!= A 0.0)
    (set `self.SteeringAngle` (`KismetMathLibrary.FClamp` (+ (* A (* (`self.DeltaT`) 140.0)) (`self.SteeringAngle`)) (* _steeringanglemax -1.0) _steeringanglemax))
    (else
      (set `self.SteeringAngle` (* (`self.SteeringAngle`) 0.9))))
  (`SceneComponent.K2_SetRelativeRotation` (`self.FL_Cup`) (`KismetMathLibrary.MakeRotator` 0.0 0.0 _steeringangle) false false)
  (`SceneComponent.K2_SetRelativeRotation` (`self.FR_Cup`) (`KismetMathLibrary.MakeRotator` 0.0 0.0 _steeringangle) false false))

(fn `SetTotalTransmissionRatio`
  (set `self.TotalTransmissionRatio` (* (`|GetArrayItem` (`self.GearRatio`) (`self.Gear`)) (`self.DifferentialRatio`))))

(fn `SetUnitMultipliers`
  (bind _output_get (set `self.RPM_RAD_multiplier` (/ (* (`KismetMathLibrary.GetPI`) 2.0) 60.0)))
  (set `self.RAD_RPM_multiplier` (/ 1.0 _output_get)))

(fn `SuspensionRay`
  (for _index (range 4)
    (bind _output (`|GetArrayItem` (`self.CupComponent`) _index))
    (bind _returnvalue (`SceneComponent.K2_GetComponentLocation` _output))
    (bind (_outhit _returnvalue_2) (`KismetSystemLibrary.LineTraceSingle` :`Start` _returnvalue :`End` (- _returnvalue (* (`SceneComponent.GetUpVector` _output) (`|GetArrayItem` (`self.RayLength`) _index))) :`TraceChannel` "TraceTypeQuery1" :`DrawDebugType` "ForDuration" :`DrawTime` 1.0))
    (`KismetArrayLibrary.Array_Set` (`self.SurfaceContact`) _index _returnvalue_2)
    (if _returnvalue_2
      (`KismetArrayLibrary.Array_Set` (`self.HitResult`) _index _outhit))))

(fn `UpdateSuspensionLength`
  (for _index (range 4)
    (if (`|GetArrayItem` (`self.SurfaceContact`) _index)
      (bind _output (`|GetArrayItem` (`self.CupComponent`) _index))
      (bind (_output_bblockinghit _output_binitialoverlap _output_time _output_distance _output_location) (`GameplayStatics.BreakHitResult` (`|GetArrayItem` (`self.HitResult`) _index)))
      (bind _output_radius (break `/Game/Cars/Miata/WheelStruct` (`|GetArrayItem` (`self.Wheel`) _index)))
      (bind (_output_restlength _output_travel) (break `/Game/Cars/Miata/SuspensionStruct` (`|GetArrayItem` (`self.Suspension`) _index)))
      (`KismetArrayLibrary.Array_Set` (`self.CurrentLength`) _index (`KismetMathLibrary.FClamp` (`KismetMathLibrary.VSize` (- (`SceneComponent.K2_GetComponentLocation` _output) (+ _output_location (* (`SceneComponent.GetUpVector` _output) _output_radius)))) (- _output_restlength _output_travel) (+ _output_restlength _output_travel)))
      (else
        (bind (_output_restlength_2 _output_travel_2) (break `/Game/Cars/Miata/SuspensionStruct` (`|GetArrayItem` (`self.Suspension`) _index)))
        (`KismetArrayLibrary.Array_Set` (`self.CurrentLength`) _index (+ _output_restlength_2 _output_travel_2))))))

(fn `UpdateWheelLocation`
  (for _index (range 4)
    (`SceneComponent.K2_SetRelativeLocation` (select `int` _index :`0` (`self.FL_Wheel`) :`1` (`self.FR_Wheel`) :`2` (`self.RL_Wheel`) :`3` (`self.RR_Wheel`)) (`KismetMathLibrary.MakeVector` 0.0 0.0 (* (`|GetArrayItem` (`self.CurrentLength`) _index) -1.0)) false false)))

(fn `UserConstructionScript`)

(fn `WheelAcceleration`
  (bind _returnvalue (select `bool` (!= (`self.Gear`) 1) :`false` 9999.0 :`true` (/ (`self.EngineAngularVelocity`) (`self.TotalTransmissionRatio`))))
  (for _index (range 4)
    (`KismetArrayLibrary.Array_Set` (`self.WheelAngularVelocity`) _index (* (`KismetMathLibrary.FMin` (`KismetMathLibrary.Abs` (+ (* (`self.DeltaT`) (/ (`|GetArrayItem` (`self.TotalTorque`) _index) (`|GetArrayItem` (`self.WheelInertia`) _index))) (`|GetArrayItem` (`self.WheelAngularVelocity`) _index))) (`KismetMathLibrary.Abs` _returnvalue)) (`KismetMathLibrary.SignOfFloat` _returnvalue)))))

(fn `WheelRotation`
  (for _index (range 4)
    (bind _output_x (`KismetMathLibrary.BreakVector` (`|GetArrayItem` (`self.WheelLinearVelocityLocal`) _index)))
    (bind _output_radius (break `/Game/Cars/Miata/WheelStruct` (`|GetArrayItem` (`self.Wheel`) _index)))
    (`SceneComponent.K2_AddLocalRotation` (select `int` _index :`0` (`self.FL_Wheel`) :`1` (`self.FR_Wheel`) :`2` (`self.RL_Wheel`) :`3` (`self.RR_Wheel`)) (`KismetMathLibrary.MakeRotator` 0.0 (* (`KismetMathLibrary.RadiansToDegrees` (* (/ _output_x (/ _output_radius 100.0)) (`self.DeltaT`))) -1.0)) false false)))